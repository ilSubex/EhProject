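; BP_TankHead is the player-controlled tank turret, handling Enhanced Input aiming and networked cannon fire.
; Look input turns the spring arm and sets a clamped target rotation, sent to the server, which Tick follows at constant speed with head yaw and cannon pitch.
; Remote shots spawn a predicted local projectile and a server one under a shared random ID.
; Tick moves local projectiles toward server counterparts, untracking pairs once they converge.
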(event Custom|SetAimRotation_Server
  (params (Rot :type Rotator))
  (Variables|Default|SetTargetRotation Rot))

(event Custom|ShootTank_Server
  (params (AimRotation :type Rotator) (IDProjectile :type Integer))
  (bind _self self)
  (Variables|Default|SetTargetRotation AimRotation)
  (Game|SpawnActorfromClass "/Game/TankArena/Blueprints/A_CannonProjectile.A_CannonProjectile_C" (Transformation|GetSocketTransform (Variables|Default|GetCannon) "Fire" "RTS_World") "AlwaysSpawn" "MultiplyWithRoot" _self IDProjectile true _self))

(event Input|EnhancedActionEvents|EnhancedInputActionIA_LookAround
  (params (ActionValue :type Vector%202D%20Structure) (ElapsedSeconds :type Float%20%28double-precision%29) (TriggeredSeconds :type Float%20%28double-precision%29) (InputAction :type Input%20Action%20Object%20Reference :default "/Game/TankArena/Input/Actions/IA_LookAround.IA_LookAround"))
  (bind (_x _y) (Math|Vector2D|BreakVector2D ActionValue))
  (Transformation|AddWorldRotation (Variables|Default|GetSpringArm) (Math|Rotator|MakeRotator 0.0 0.0 _x) false false)
  (Variables|Default|SetTargetRotation (CallFunction|CalculateAimRotation _y))
  (Networking|SwitchHasAuthority
    (:Remote
      (CallFunction|SetAimRotationServer (Variables|Default|GetTargetRotation)))))

(event Input|EnhancedActionEvents|EnhancedInputActionIA_ShootTank
  (params (ActionValue :type Boolean) (ElapsedSeconds :type Float%20%28double-precision%29) (TriggeredSeconds :type Float%20%28double-precision%29) (InputAction :type Input%20Action%20Object%20Reference :default "/Game/TankArena/Input/Actions/IA_ShootTank.IA_ShootTank"))
  (bind _self self)
  (bind _self_2 self)
  (:Started
    (Networking|SwitchHasAuthority
      (:Authority
        (Game|SpawnActorfromClass "/Game/TankArena/Blueprints/A_CannonProjectile.A_CannonProjectile_C" (Transformation|GetSocketTransform (Variables|Default|GetCannon) "Fire" "RTS_World") "AlwaysSpawn" "MultiplyWithRoot" _self_2 0 true _self_2))
      (:Remote
        (Variables|Default|SetIDProjectile (CallFunction|GenerateID))
        (CallFunction|ShootTankServer (Math|Rotator|MakeRotator 0.0 (Variables|Default|GetCurrentCannoRotation) (Variables|Default|GetcurrentHeadRotation)) (Variables|Default|GetIDProjectile))
        (bind _returnvalue (Game|SpawnActorfromClass "/Game/TankArena/Blueprints/A_CannonProjectile.A_CannonProjectile_C" (Transformation|GetSocketTransform (Variables|Default|GetCannon) "Fire" "RTS_World") "AlwaysSpawn" "MultiplyWithRoot" _self (Variables|Default|GetIDProjectile) false _self))
        (Utilities|Map|Add (Variables|Default|GetClientProjectilesMap) (Variables|Default|GetIDProjectile) _returnvalue)))))

(event EventBeginPlay)

(event Collision|EventActorBeginOverlap
  (params (OtherActor :type Actor%20Object%20Reference)))

(event EventControllerChanged
  (params (OldController :type Controller%20Object%20Reference) (NewController :type Controller%20Object%20Reference))
  (Utilities|IsValid NewController
    (:Is%20Valid
      (bind _asplayer_controller (Utilities|Casting|CastToPlayerController NewController))
      (Utilities|IsValid (PlayerController|LocalPlayerSubsystems|GetEnhancedInputLocalPlayerSubsystem _asplayer_controller)
        (:Is%20Valid
          (Input|AddMappingContext (PlayerController|LocalPlayerSubsystems|GetEnhancedInputLocalPlayerSubsystem _asplayer_controller) "/Game/TankArena/Input/IMC_TankControls.IMC_TankControls" 0 "(bIgnoreAllPressedKeysUntilRelease=True,bForceImmediately=False,bNotifyUserSettings=False)"))))))

(event EventTick
  (params (DeltaSeconds :type Float%20%28single-precision%29))
  (Utilities|FlowControl|Sequence
    (:then_0
      (Variables|Default|SetcurrentHeadRotation (.yaw (Class|KismetMathLibrary|RInterptoConstant (Math|Rotator|MakeRotator 0.0 0.0 (Variables|Default|GetcurrentHeadRotation)) (Math|Rotator|MakeRotator 0.0 0.0 (.yaw (Variables|Default|GetTargetRotation))) (Utilities|Time|GetWorldDeltaSeconds) 5e+01)))
      (Transformation|SetWorldRotation (Variables|Default|GetHead) (Math|Rotator|MakeRotator 0.0 0.0 (Variables|Default|GetcurrentHeadRotation)) false false))
    (:then_1
      (Variables|Default|SetCurrentCannoRotation (Math|Interpolation|FInterptoConstant (Variables|Default|GetCurrentCannoRotation) (.pitch (Variables|Default|GetTargetRotation)) (Utilities|Time|GetWorldDeltaSeconds) 5e+01))
      (Transformation|SetRelativeRotation (Variables|Default|GetCannon) (Math|Rotator|MakeRotator 0.0 (Variables|Default|GetCurrentCannoRotation) 0.0) false false))
    (:then_2
      ;[0.15 0.15 0.15 0.5 50] Sync projectiles tick if both list has one item and this item are the same id
      (if (and (> (Utilities|Map|Length (Variables|Default|GetServerProjectilesMap)) 0) (> (Utilities|Map|Length (Variables|Default|GetClientProjectilesMap)) 0))
        (bind _keys (Utilities|Map|Keys (Variables|Default|GetClientProjectilesMap)))
        (bind _keys_2 (Utilities|Map|Keys (Variables|Default|GetServerProjectilesMap)))
        (bind _array_element (Utilities|Array|ForEachLoopwithBreak _keys)
          (:LoopBody
            (if (Utilities|Array|ContainsItem _keys_2 _array_element)
              (if (.ReturnValue (Utilities|Map|Find (Variables|Default|GetClientProjectilesMap) _array_element))
                (if (.ReturnValue (Utilities|Map|Find (Variables|Default|GetServerProjectilesMap) _array_element))
                  (Transformation|SetActorLocation (.Value (Utilities|Map|Find (Variables|Default|GetClientProjectilesMap) _array_element)) (Math|Interpolation|VInterptoConstant (Transformation|GetActorLocation (.Value (Utilities|Map|Find (Variables|Default|GetClientProjectilesMap) _array_element))) (Transformation|GetActorLocation (.Value (Utilities|Map|Find (Variables|Default|GetServerProjectilesMap) _array_element))) (Utilities|Time|GetWorldDeltaSeconds) 5e+02) false false)
                  (if (Utilities|Operators|EqualEqual (Transformation|GetActorLocation (.Value (Utilities|Map|Find (Variables|Default|GetClientProjectilesMap) _array_element))) (Transformation|GetActorLocation (.Value (Utilities|Map|Find (Variables|Default|GetServerProjectilesMap) _array_element))) 1e+01)
                    (CallFunction|RemoveProjectile _array_element)))))))))))

(fn ConstructionScript)

(fn CalculateAimRotation
  (params (B :type Float%20%28double-precision%29))
  (return (Math|Rotator|MakeRotator 0.0 (Math|Float|Clamp(Float) (+ B (.pitch (Variables|Default|GetTargetRotation))) 0.0 3e+01) (.yaw (Transformation|GetWorldRotation (Variables|Default|GetSpringArm))))))

(fn GenerateID
  (return (Math|Random|RandomInteger 1000)))

(fn SyncProjectiles
  (params (ID :type Integer) (newProjectile :type A%20Cannon%20Projectile%20Object%20Reference))
  (if (.ReturnValue (Utilities|Map|Find (Variables|Default|GetClientProjectilesMap) ID))
    (Utilities|Map|Add (Variables|Default|GetServerProjectilesMap) ID newProjectile)))

(fn RemoveProjectile
  (params (ID :type Integer))
  (Utilities|Map|Remove (Variables|Default|GetClientProjectilesMap) ID)
  (Utilities|Map|Remove (Variables|Default|GetServerProjectilesMap) ID))
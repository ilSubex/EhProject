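; Game mode for TankArena that puts joining players into two-person tanks.
; On PostLogin a FlipFlop alternates roles: one player possesses a new CH_TankBody, the next possesses a BP_TankHead attached to that body's Head socket.
; Bodies spawn at a RED-tagged PlayerStart with no tank body overlapping it, falling back to a random start.
; Player starts are cached on BeginPlay, or at login if still empty.
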(event EventBeginPlay
  (SpawnLogic|GetAllPlayerStarts))

(event EventTick
  (params (DeltaSeconds :type Float%20%28single-precision%29)))

(event EventPostLogin
  (params (NewPlayer :type Player%20Controller%20Object%20Reference))
  (bind _output_get (Variables|Default|SetLastLoggedPc NewPlayer))
  (if (Utilities|Array|IsValidIndex (Variables|Default|GetPlayerStartsArray))
    _
    (else
      (SpawnLogic|GetAllPlayerStarts)))
  (Utilities|Array|Add (Variables|Default|GetPlayerControllers) _output_get)
  (Utilities|FlowControl|FlipFlop
    (:A
      (bind _returnvalue (Game|SpawnActorfromClass "/Game/TankArena/Blueprints/CH_TankBody.CH_TankBody_C" (Transformation|GetActorTransform (CallFunction|GetFreeSpawnPointbyTeam "RED")) "Undefined" "MultiplyWithRoot" 0 0))
      (bind _output_get_2 (Variables|Default|SetLastSpawnTankBody _returnvalue))
      (Pawn|Possess (Variables|Default|GetLastLoggedPc) _output_get_2))
    (:B
      (bind _returnvalue_2 (Game|SpawnActorfromClass "/Game/TankArena/Blueprints/BP_TankHead.BP_TankHead_C" (Transformation|GetSocketTransform (Variables|/Game/TankArena/Blueprints/CH_TankBody.CH_TankBody_C|GetBody (Variables|Default|GetLastSpawnTankBody)) "Head" "RTS_ParentBoneSpace") "AlwaysSpawn" "MultiplyWithRoot" 0 0))
      (Transformation|AttachComponentToComponent _returnvalue_2 (Variables|/Game/TankArena/Blueprints/CH_TankBody.CH_TankBody_C|GetBody (Variables|Default|GetLastSpawnTankBody)) "Head" "KeepRelative" "KeepRelative" "KeepRelative" true)
      (Pawn|Possess (Variables|Default|GetLastLoggedPc) _returnvalue_2))))

(fn ConstructionScript)

(fn GetFreeSpawnPointbyTeam
  (params (TeamTag :type Name))
  (for _array_element (Variables|Default|GetPlayerStartsArray)
    (LocalVariables|SettmpStart _array_element)
    (if (== (Variables|/Script/Engine.PlayerStart|GetPlayerStartTag _array_element) TeamTag)
      (bind _returnvalue (Collision|SphereOverlapActors (Transformation|GetActorLocation _array_element) 1e+02 (Utilities|Array|MakeArray "ObjectTypeQuery3") "/Game/TankArena/Blueprints/CH_TankBody.CH_TankBody_C" (Utilities|Array|MakeArray _array_element)))
      (if (not _returnvalue)
        (return (LocalVariables|GettmpStart)))))
  (return (.OutItem (Utilities|Array|Random (Variables|Default|GetPlayerStartsArray)))))

(fn GetAllPlayerStarts
  (bind _outactors (Actor|GetAllActorsOfClass "/Script/Engine.PlayerStart"))
  (Variables|Default|SetPlayerStartsArray _outactors))
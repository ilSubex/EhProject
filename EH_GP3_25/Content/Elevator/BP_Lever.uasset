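; BP_Lever is an interactive lever that triggers a linked sliding door, DoorToSlide.
; Trigger passes a DoOnce gate and plays or reverses the LeverMove timeline based on LeverDirection, rotating the Cylinder; finishing resets the gate.
; A timeline event track triggers the door directly on authority or through RequestOpenDoorServer on remotes.
; Only authority records LeverDirection during timeline updates.
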(event Custom|ResetLever
  (Utilities|FlowControl|DoOnce false) ; enters at Reset
)

(event Custom|RequestOpenDoorServer
  (Default|Trigger (Variables|Default|GetDoorToSlide)))

(event EventBeginPlay)

(event Collision|EventActorBeginOverlap
  (params (OtherActor :type Actor%20Object%20Reference)))

(event EventTick
  (params (DeltaSeconds :type Float%20%28single-precision%29)))

(event EventTrigger
  (params (Instigator :type Pawn%20Object%20Reference))
  (Utilities|FlowControl|DoOnce false
    (:Completed
      (switch Utilities|FlowControl|Switch|SwitchonETimelineDirection (Variables|Default|GetLeverDirection)
        (:Forward
          (Utilities|String|Reverse (Variables|Default|GetLeverMove)))
        (:Backward
          (Audio|Components|Audio|Play (Variables|Default|GetLeverMove)))))))

(fn ConstructionScript)

(fn GetTargetUI
  (return 0 0))
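; Elevator actor that travels between three floors, with its starting location as the first.
; Elevator calls branch on authority: the server moves directly, while remote callers invoke RequestMoveElevator to request the move.
; If not already at the chosen floor, it plays the slowed MoveTo timeline, whose graph lerps from the current location to the target and dings on finish.
; Debug prints trace each step.
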(event Custom|RequestMoveElevator
  (params (Instigator :type Pawn%20Object%20Reference))
  (bind _moveto (Variables|Default|GetMoveTo))
  (Development|PrintString "call server")
  (if (Utilities|Operators|NotEqual(!=) (Transformation|GetActorLocation) (Utilities|Array|Get(acopy) (Variables|Default|GetFloors) (stale EventElevator indexFloor)) 1.0)
    (Development|PrintString "different location")
    (Variables|Default|SetTarget (Utilities|Array|Get(acopy) (Variables|Default|GetFloors) (stale EventElevator indexFloor)))
    (Components|Timeline|SetPlayRate _moveto 0.05)
    (Components|Timeline|PlayfromStart _moveto)
    (Development|PrintString "call timeline")
    (else
      (Development|PrintString "same location"))))

(event EventBeginPlay
  (Variables|Default|SetFirstFloor (Transformation|GetActorLocation))
  (Variables|Default|SetFloors (Utilities|Array|MakeArray (Variables|Default|GetFirstFloor) (Variables|Default|GetSecondFloor) (Variables|Default|GetThirdFloor))))

(event Collision|EventActorBeginOverlap
  (params (OtherActor :type Actor%20Object%20Reference)))

(event EventTick
  (params (DeltaSeconds :type Float%20%28single-precision%29)))

(event EventElevator
  (params (indexFloor :type Integer) (Instigator :type Pawn%20Object%20Reference))
  (bind _floors (Variables|Default|GetFloors))
  (bind _moveto (Variables|Default|GetMoveTo))
  (bind _output (Utilities|Array|Get(acopy) _floors indexFloor))
  (Networking|SwitchHasAuthority
    (:Authority
      (Development|PrintString "call elevator")
      (if (Utilities|Operators|NotEqual(!=) (Transformation|GetActorLocation) _output 1.0)
        (Development|PrintString "different location")
        (Variables|Default|SetTarget _output)
        (Components|Timeline|SetPlayRate _moveto 0.05)
        (Components|Timeline|PlayfromStart _moveto)
        (Development|PrintString "call timeline")
        (else
          (Development|PrintString "same location"))))
    (:Remote
      (CallFunction|RequestMoveElevator)
      (Development|PrintString "from client"))))

(fn ConstructionScript)

(fn GetTargetUI
  (return 0 0))
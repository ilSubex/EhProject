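; Actor component that lets its owning BP_FirstPersonCharacter interact with the actor it looks at.
; Interaction runs a short, debug-drawn sphere trace forward from the first-person camera on the Visibility channel.
; A hit actor receives TriggerMessage with the character, called directly on authority or through RequestInteractionServer on remote.
; InteractionPanelElevator is an empty stub.
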(event Custom|RequestInteractionServer
  (params (ObjectRef :type Actor%20Object%20Reference))
  (Class|BPITriggerable|Trigger(Message) ObjectRef (Variables|Default|GetAs%20BP%20First%20Person%20Character)))

(event EventBeginPlay
  (bind _asbp_first_person_character (Utilities|Casting|CastToBP_FirstPersonCharacter (Components|GetOwner)))
  (Variables|Default|SetAs%20BP%20First%20Person%20Character _asbp_first_person_character))

(event EventTick
  (params (DeltaSeconds :type Float%20%28single-precision%29)))

(fn InteractionPanelElevator
  (params (Elevator :type Actor%20Object%20Reference) (Widget :type User%20Widget%20Class%20Reference)))

(fn Interaction
  (bind _as_bp_first_person_character (Variables|Default|GetAs%20BP%20First%20Person%20Character))
  (bind _firstpersoncameracomponent (Variables|/Script/EH_GP3_25.EH_GP3_25Character|GetFirstPersonCameraComponent _as_bp_first_person_character))
  (bind _returnvalue (Transformation|GetWorldLocation _firstpersoncameracomponent))
  (bind (_outhit _returnvalue_2) (Collision|SphereTraceByChannel _returnvalue (+ _returnvalue (* (Math|Vector|GetForwardVector _firstpersoncameracomponent) 1.5e+02)) 25.0 "TraceTypeQuery1" false 0 "ForOneFrame"))
  (if _returnvalue_2
    (Networking|SwitchHasAuthority
      (:Authority
        (Class|BPITriggerable|Trigger(Message) (.hitactor _outhit) (Variables|Default|GetAs%20BP%20First%20Person%20Character)))
      (:Remote
        (CallFunction|RequestInteractionServer (.hitactor _outhit))))))
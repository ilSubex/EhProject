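; BP_Door is an elevator-folder door that slides a cube vertically, toggling between open and closed each time it is triggered.
; The Trigger event prints a debug string, then a FlipFlop alternates between playing and reversing the Sliding timeline.
; The timeline's Alpha is meant to lerp the Cube's relative Z between two heights.
; GetTargetUI is an empty stub.
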(event EventBeginPlay)

(event Collision|EventActorBeginOverlap
  (params (OtherActor :type Actor%20Object%20Reference)))

(event EventTick
  (params (DeltaSeconds :type Float%20%28single-precision%29)))

(event EventTrigger
  (params (Instigator :type Pawn%20Object%20Reference))
  (Development|PrintString "call door")
  (Utilities|FlowControl|FlipFlop
    (:A
      (Audio|Components|Audio|Play (Variables|Default|GetSliding)))
    (:B
      (Utilities|String|Reverse (Variables|Default|GetSliding)))))

(fn ConstructionScript)

(fn GetTargetUI
  (return 0 0))
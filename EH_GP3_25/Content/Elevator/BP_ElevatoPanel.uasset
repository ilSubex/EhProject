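; Elevator panel actor that opens the elevator UI when triggered, working as a child actor of its parent elevator.
; Trigger runs only on authority, casts the instigator to BP_FirstPersonCharacter and asks it to spawn BPW_Elevator with the parent actor as the elevator.
; GetTargetUI reports that same parent and widget class, while older direct widget-creation and input-mode logic remains unconnected.
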(event EventBeginPlay)

(event Collision|EventActorBeginOverlap
  (params (OtherActor :type Actor%20Object%20Reference)))

(event EventTick
  (params (DeltaSeconds :type Float%20%28single-precision%29)))

(event EventTrigger
  (params (Instigator :type Pawn%20Object%20Reference))
  (Networking|SwitchHasAuthority
    (:Authority
      (bind _asbp_first_person_character (Utilities|Casting|CastToBP_FirstPersonCharacter Instigator))
      (Default|SpawnUI _asbp_first_person_character "/Game/Elevator/BPW_Elevator.BPW_Elevator_C" 1 (Actor|GetParentActor)))))

(fn ConstructionScript)

(fn GetTargetUI
  (return (Actor|GetParentActor) "/Game/Elevator/BPW_Elevator.BPW_Elevator_C"))